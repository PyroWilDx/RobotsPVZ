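; BP_Zombie is an AI enemy that chases a target Character.
; BeginPlay starts a short Delay loop that reissues MoveToActor through the AI controller, holding off while IsBeingHurt is true.
; Tick rotates the zombie toward the Character using a look-at rotation with a yaw offset.
; Tick also disables movement while the zombie is being hurt and otherwise sets it back to walking.
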(event `self.ReceiveBeginPlay`
  (`AIController.MoveToActor` (`AIBlueprintHelperLibrary.GetAIController` self) (`self.Character`) -1.0 true true true null true :!label _label)
  (`KismetSystemLibrary.Delay` 0.2 :!label _label_2)
  (if (`self.IsBeingHurt`)
    (goto _label_2)
    (else
      (goto _label))))

(event `self.ReceiveTick`
  (params (DeltaSeconds :type "Float (single-precision)"))
  (bind _charactermovement (`self.CharacterMovement`))
  (`self.K2_SetActorRotation` self (`KismetMathLibrary.MakeRotator` (.roll (`KismetMathLibrary.FindLookAtRotation` (`self.K2_GetActorLocation` self) (`self.K2_GetActorLocation` (`self.Character`)))) (.pitch (`KismetMathLibrary.FindLookAtRotation` (`self.K2_GetActorLocation` self) (`self.K2_GetActorLocation` (`self.Character`)))) (- (.yaw (`KismetMathLibrary.FindLookAtRotation` (`self.K2_GetActorLocation` self) (`self.K2_GetActorLocation` (`self.Character`)))) 90.0)) false)
  (if (`self.IsBeingHurt`)
    (`CharacterMovementComponent.DisableMovement` _charactermovement)
    (else
      (`CharacterMovementComponent.SetMovementMode` _charactermovement "MOVE_Walking" 0))))

(fn `UserConstructionScript`)